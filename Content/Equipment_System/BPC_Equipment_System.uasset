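; Player equipment component that picks up weapons in the world and opens the equipment menu.
; Interact sphere-traces from the follow camera, stores the hit BP_Weapon's item data in WeaponSlots and destroys the actor.
; The menu input toggles WB_Equipment, switching cursor and input mode, blocking attacks through the combat component and disabling character movement while open.
; A debug key prints the stored weapon row names.
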(event Input|EnhancedActionEvents|EnhancedInputActionIA_Interact
  (params (ActionValue :type Boolean) (ElapsedSeconds :type Float%20%28double-precision%29) (TriggeredSeconds :type Float%20%28double-precision%29) (InputAction :type Input%20Action%20Object%20Reference :default "/Game/ThirdPerson/Input/Actions/IA_Interact.IA_Interact"))
  (bind _follow_camera (Variables|Default|GetFollow%20Camera))
  (bind _returnvalue (Transformation|GetWorldLocation _follow_camera))
  ;[1 1 1] Pick & Trace
  (:Started
    (bind (_outhit _returnvalue_2) (Collision|SphereTraceForObjects _returnvalue (+ _returnvalue (* (Math|Vector|GetForwardVector (Transformation|GetWorldRotation _follow_camera)) 1e+03)) 15.0 (Utilities|Array|MakeArray "ObjectTypeQuery2") false 0 "ForDuration"))
    (if _returnvalue_2
      (bind _asbp_weapon (Utilities|Casting|CastToBP_Weapon (.HitActor (Collision|BreakHitResult _outhit))))
      (CallFunction|AddWeapon (Variables|/Game/Equipment_System/BP_Weapon.BP_Weapon_C|GetItem%20Data _asbp_weapon))
      (Actor|DestroyActor _asbp_weapon)
      (Development|PrintString "Item Picked"))))

(event Input|EnhancedActionEvents|EnhancedInputActionIA_OpenManu
  (params (ActionValue :type Boolean) (ElapsedSeconds :type Float%20%28double-precision%29) (TriggeredSeconds :type Float%20%28double-precision%29) (InputAction :type Input%20Action%20Object%20Reference :default "/Game/ThirdPerson/Input/Actions/IA_OpenManu.IA_OpenManu"))
  (bind _returnvalue (Game|GetPlayerController 0))
  (bind _bpc_combat_system (Variables|Default|GetBPC%20Combat%20System))
  ;[1 1 1] Equipment Manu
  (:Started
    (if (not (Variables|Default|GetIs%20Manu%20opened?))
      (Variables|/Game/Base_data/BPC_Combat_System.BPC_Combat_System_C|SetCan%20Attack? _bpc_combat_system false)
      (Variables|Default|SetIs%20Manu%20opened? true)
      (bind _returnvalue_2 (UserInterface|CreateWidget "/Game/Equipment_System/UI/WB_Equipment.WB_Equipment_C"))
      (bind _output_get (Variables|Default|SetEquipment%20Widgets _returnvalue_2))
      (UserInterface|Viewport|AddtoViewport _output_get 0)
      (Variables|/Script/Engine.PlayerController|SetbShowMouseCursor _returnvalue true)
      (Input|SetInputModeGameandUI _returnvalue (Variables|Default|GetEquipment%20Widgets) "DoNotLock" true false)
      (bind _asbp_third_person_character (Utilities|Casting|CastToBP_ThirdPersonCharacter (Components|GetOwner)))
      (Pawn|Components|CharacterMovement|SetMovementMode (Variables|/Script/Engine.Character|GetCharacterMovement _asbp_third_person_character) "MOVE_None" 0)
      (else
        (Variables|/Game/Base_data/BPC_Combat_System.BPC_Combat_System_C|SetCan%20Attack? _bpc_combat_system true)
        (Variables|Default|SetIs%20Manu%20opened? false)
        (bind _equipment_widgets (Variables|Default|GetEquipment%20Widgets)
          (:then
            (Widget|RemovefromParent _equipment_widgets)
            (Variables|Default|SetEquipment%20Widgets 0)
            (Variables|/Script/Engine.PlayerController|SetbShowMouseCursor _returnvalue false)
            (Input|SetInputModeGameOnly _returnvalue false)
            (bind _asbp_third_person_character_2 (Utilities|Casting|CastToBP_ThirdPersonCharacter (Components|GetOwner)))
            (Pawn|Components|CharacterMovement|SetMovementMode (Variables|/Script/Engine.Character|GetCharacterMovement _asbp_third_person_character_2) "MOVE_Walking" 0))
          (:else))))))

(event EventBeginPlay
  (bind _asbp_third_person_character (Utilities|Casting|CastToBP_ThirdPersonCharacter (Components|GetOwner)))
  (Variables|Default|SetFollow%20Camera (Variables|/Game/ThirdPerson/Blueprints/BP_ThirdPersonCharacter.BP_ThirdPersonCharacter_C|GetFollowCamera _asbp_third_person_character))
  (Variables|Default|SetBPC%20Combat%20System (Variables|/Game/ThirdPerson/Blueprints/BP_ThirdPersonCharacter.BP_ThirdPersonCharacter_C|GetBPC_Combat_System _asbp_third_person_character)))

(event Input|KeyboardEvents|DebugKeyH
  (params (Key :type Key%20Structure :default "None") (ActionValue :type Input%20Action%20Value%20Structure))
  (:Pressed
    (for _array_element (Variables|Default|GetWeapon%20Slots)
      (Development|PrintString (Utilities|String|ToString(Name) (.rowname (.item _array_element)))))))

(fn AddWeapon
  (params (NewItem :type S%20Slots%20Structure%20%28by%20ref%29))
  (Utilities|Array|Add (Variables|Default|GetWeapon%20Slots) NewItem))