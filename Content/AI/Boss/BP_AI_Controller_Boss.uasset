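; AI controller for a boss that runs the BT_AI_Boss behavior tree and manages the boss's on-screen health bar.
; The behavior tree starts on BeginPlay, while Activate_Boss creates the health bar widget and adds it to the viewport.
; Tick sets the bar from Health over MaxHealth whenever the widget is valid.
; Deactivate_Boss only hides the widget; its removal and reference-clearing nodes are never run.
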(event `self.ReceiveBeginPlay`
  (`self.RunBehaviorTree` "/Game/AI/Boss/BT_AI_Boss.BT_AI_Boss"))

(event `Activate_Boss`
  (bind _returnvalue (`|CreateWidget` "/Game/UI/WB_Boss_Healthbar.WB_Boss_Healthbar_C"))
  (bind _output_get (set `self.Boss HP Bar Widget` _returnvalue))
  (`UserWidget.AddToViewport` _output_get 0))

(event `Deactivate_Boss`
  (`Widget.SetVisibility` (`self.Boss HP Bar Widget`) "Hidden"))

(event `self.ReceiveTick`
  (params (DeltaSeconds :type "Float (single-precision)"))
  (bind _boss_hp_bar_widget (`self.Boss HP Bar Widget`)
    (:`then`
      (`ProgressBar.SetPercent` (`/Game/UI/WB_Boss_Healthbar.HealthBar` _boss_hp_bar_widget) (/ (`self.Health`) (`self.MaxHealth`))))
    (:`else`)))

(fn `UserConstructionScript`
  (`parent.UserConstructionScript`))