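; Enemy AI character that fights with sword combos and can be stealth-assassinated from behind.
; Behavior-tree attacks chain montages through an index and saved-attack flag, dealing damage via a timer-looped sword trace or single sphere trace.
; Damage interrupts combos, triggers hit reactions and launches, then ragdolls on death through the stats component.
; Assassination returns alignment to the caller and ragdolls after a delay; prompt, health and investigate widgets face the camera.
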(event `self.ReceiveBeginPlay`
  (bind _aswb_dummy_health_bar (cast `/Game/UI/WB_Dummy_HealthBar` (`WidgetComponent.GetWidget` (`self.Health Bar Widget`))))
  (set `self.Health Bar UI` _aswb_dummy_health_bar))

(event `self.ReceiveTick`
  (params (DeltaSeconds :type "Float (single-precision)"))
  (`SceneComponent.K2_SetWorldRotation` (`self.Assasinate Widget`) (`KismetMathLibrary.FindLookAtRotation` (`SceneComponent.K2_GetComponentLocation` (`self.Assasinate Widget`)) (`SceneComponent.K2_GetComponentLocation` (`Actor.RootComponent` (`GameplayStatics.GetPlayerCameraManager` 0)))) false false)
  (`SceneComponent.K2_SetWorldRotation` (`self.Health Bar Widget`) (`KismetMathLibrary.FindLookAtRotation` (`SceneComponent.K2_GetComponentLocation` (`self.Assasinate Widget`)) (`SceneComponent.K2_GetComponentLocation` (`Actor.RootComponent` (`GameplayStatics.GetPlayerCameraManager` 0)))) false false)
  (`SceneComponent.K2_SetWorldRotation` (`self.investigate_Widget`) (`KismetMathLibrary.FindLookAtRotation` (`SceneComponent.K2_GetComponentLocation` (`self.Assasinate Widget`)) (`SceneComponent.K2_GetComponentLocation` (`Actor.RootComponent` (`GameplayStatics.GetPlayerCameraManager` 0)))) false false))

(event `Regdoll`
  ;[1 1 1] Ragdoll
  (`|ExecutionSequence`
    (:`then_0`
      (`KismetSystemLibrary.Delay` 2.5)
      (`PrimitiveComponent.SetSimulatePhysics` (`self.Mesh`) true))
    (:`then_1`
      (`KismetSystemLibrary.Delay` 1.5)
      (`GameplayStatics.PlaySoundAtLocation` "/Game/Audio/Hits_Sounds/SC_Death.SC_Death" (`self.K2_GetActorLocation`) (struct) 1.0 1.0 0.0 "/Game/Audio/SA_Character.SA_Character" null null null))))

(event `self.Assasin Area.OnComponentBeginOverlap`
  (params (OverlappedComponent :type "PrimitiveComponent Object Reference") (OtherActor :type "Actor Object Reference") (OtherComp :type "PrimitiveComponent Object Reference") (OtherBodyIndex :type Integer) (bFromSweep :type Boolean) (SweepResult :type "HitResult Structure (by ref)"))
  (cast `/Game/ThirdPerson/Blueprints/BP_ThirdPersonCharacter` OtherActor)
  (`SceneComponent.SetVisibility` (`self.Assasinate Widget`) true false))

(event `self.Assasin Area.OnComponentEndOverlap`
  (params (OverlappedComponent :type "PrimitiveComponent Object Reference") (OtherActor :type "Actor Object Reference") (OtherComp :type "PrimitiveComponent Object Reference") (OtherBodyIndex :type Integer))
  (cast `/Game/ThirdPerson/Blueprints/BP_ThirdPersonCharacter` OtherActor)
  (`SceneComponent.SetVisibility` (`self.Assasinate Widget`) false false))

(event `self.ReceiveAnyDamage`
  (params (Damage :type "Float (single-precision)") (DamageType :type "DamageType Object Reference") (InstigatedBy :type "Controller Object Reference") (DamageCauser :type "Actor Object Reference"))
  (`self.Stop Combo`)
  (`self.PlayAnimMontage` (`|GetArrayItem` (`self.Hit index`) (`KismetMathLibrary.RandomIntegerInRange` 0 (- (`KismetArrayLibrary.Array_Length` (`self.Hit index`)) 1))))
  (bind _asbp_third_person_character (cast `/Game/ThirdPerson/Blueprints/BP_ThirdPersonCharacter` (`GameplayStatics.GetPlayerCharacter` 0)))
  (`self.LaunchCharacter` (* (`KismetMathLibrary.GetForwardVector` (`self.K2_GetActorRotation` _asbp_third_person_character)) 800.0))
  (`GameplayStatics.PlaySoundAtLocation` "/Game/Audio/Hits_Sounds/Death1.Death1" (`self.K2_GetActorLocation`) (struct) 1.0 (`KismetMathLibrary.RandomFloatInRange` 0.8 1.2) 0.0 "/Game/Audio/SA_Character.SA_Character" null null null)
  (bind _is_player_dead (`/Game/Base_data/BPC_PlayerStats.Decrease Health` (`self.BPC_PlayerStats`) Damage))
  (if _is_player_dead
    (`PrimitiveComponent.SetCollisionObjectType` (`self.Mesh`) "ECC_PhysicsBody")
    (`PrimitiveComponent.SetSimulatePhysics` (`self.Mesh`) true)
    (`GameplayStatics.PlaySoundAtLocation` "/Game/Audio/Hits_Sounds/SC_Death.SC_Death" (`self.K2_GetActorLocation`) (struct) 1.0 1.0 0.0 "/Game/Audio/SA_Character.SA_Character" null null null)
    (`SceneComponent.SetVisibility` (`self.Health Bar Widget`) false false)))

(event `Attack1`
  ;[1 1 1] combo
  ;;[0.4583 0 0.02547] Attack1
  (`/Engine/EditorBlueprintResources/StandardMacros.DoOnce` false :!label _label
    (:`Completed`
      (`KismetSystemLibrary.Delay` 0.1)
      (`|PlayMontage` (`self.Mesh`) "/Game/Characters/RPG_Characters/Animation/Attack_Sword/Attack1_Montage.Attack1_Montage" (`self.Attack Speed`)
        (:`then`
          (set `self.Index_attack` 1)
          (goto _label :!via `Reset`))))))

(event `SwordAttackFromBT_AI`
  ;[1 1 1] combo
  ;;[0.05127 0.05127 0.05127] Normal Attack
  (if (`self.Can Attack?`)
    (`self.Attack Sward`)))

(event `Attack2`
  ;[1 1 1] combo
  ;;[0.4583 0 0.02547] Attack2
  (`/Engine/EditorBlueprintResources/StandardMacros.DoOnce` false :!label _label_2
    (:`Completed`
      (`KismetSystemLibrary.Delay` 0.1)
      (`|PlayMontage` (`self.Mesh`) "/Game/Characters/RPG_Characters/Animation/Attack_Sword/Attack2_Montage.Attack2_Montage" (`self.Attack Speed`)
        (:`then`
          (set `self.Index_attack` 2)
          (goto _label_2 :!via `Reset`))))))

(event `Attack Sward`
  ;[1 1 1] combo
  ;;[1 0.1042 0.1042] Sword Attack
  (if (`self.Attacking?`)
    (set `self.Save Attack?` true)
    (else
      (set `self.Attacking?` true)
      (switch `int` (`self.Index_attack`) :!label _label_3
        (:`0`
          (`self.Attack1`))
        (:`1`
          (`self.Attack2`))
        (:`2`
          (`self.Attack4`))))))

(event `Attack3`
  ;[1 1 1] combo
  ;;[0.4583 0 0.02547] Attack3
  (`/Engine/EditorBlueprintResources/StandardMacros.DoOnce` false :!label _label_4
    (:`Completed`
      (`KismetSystemLibrary.Delay` 0.1)
      (`|PlayMontage` (`self.Mesh`) "/Game/Characters/RPG_Characters/Animation/Attack_Sword/Kick_Montage.Kick_Montage" (`self.Attack Speed`)
        (:`then`
          (set `self.Index_attack` 3)
          (goto _label_4 :!via `Reset`))))))

(event `Attack Combo_Sward`
  ;[1 1 1] combo
  ;;[1 0.1042 0.1042] Sword Attack
  (if (`self.Save Attack?`)
    (set `self.Save Attack?` false)
    (goto _label_3)
    (else
      (`self.Stop Combo`))))

(event `Attack4`
  ;[1 1 1] combo
  ;;[0.4583 0 0.02547] Attack4
  (`/Engine/EditorBlueprintResources/StandardMacros.DoOnce` false :!label _label_5
    (:`Completed`
      (`KismetSystemLibrary.Delay` 0.1)
      (`|PlayMontage` (`self.Mesh`) "/Game/Characters/RPG_Characters/Animation/Attack_Sword/Attack3_Montage.Attack3_Montage" (`self.Attack Speed`)
        (:`then`
          (set `self.Index_attack` 4)
          (goto _label_5 :!via `Reset`))))))

(event `Stop Combo`
  ;[1 1 1] combo
  ;;[0.05127 0.05127 0.05127] Stop Combo
  (set `self.Attacking?` false)
  (set `self.Index_attack` 0))

(event `Sword Trace start`
  ;[1 0.3372 0.3372] Sword Trace
  (bind _returnvalue (`KismetSystemLibrary.K2_SetTimerDelegate` (delegate `Sword Trace Loop`) 0.001 true))
  (set `self.Sword_Trace_Loop` _returnvalue))

(event `Sword Trace Loop`
  ;[1 0.3372 0.3372] Sword Trace
  (bind (_outhit _returnvalue) (`KismetSystemLibrary.SphereTraceSingle` :`Start` (`SceneComponent.K2_GetComponentLocation` (`self.Sword Top`)) :`End` (`SceneComponent.K2_GetComponentLocation` (`self.Sword Bottom`)) :`Radius` 12.0 :`TraceChannel` "TraceTypeQuery1" :`DrawDebugType` "ForDuration" :`DrawTime` 0.5))
  (if _returnvalue
    (bind (_bblockinghit _binitialoverlap _time _distance _location _impactpoint _normal _impactnormal _physmat _hitactor) (`GameplayStatics.BreakHitResult` _outhit))
    (if (`self.ActorHasTag` _hitactor "Damageable")
      (`/Engine/EditorBlueprintResources/StandardMacros.DoOnce` false :!label _label_6
        (:`Completed`
          (`GameplayStatics.ApplyDamage` _hitactor 10.0)
          (`GameplayStatics.PlayWorldCameraShake` "/Game/Base_data/BP_CameraShake_受击.BP_CameraShake_受击_C" _location 0.0 2000.0)
          (`self.Play Sword hit sound`)
          (`GameplayStatics.SpawnEmitterAtLocation` "/Game/Effect_Particle/Particles/Blood/P_Blood_Splat_Cone.P_Blood_Splat_Cone" _location (`KismetMathLibrary.MakeRotFromXY` _normal _normal) (0.4 0.4 0.4) true "AutoRelease")
          (`KismetSystemLibrary.Delay` 0.5)
          (goto _label_6 :!via `Reset`))))))

(event `Swrod Trace Stop`
  ;[1 0.3372 0.3372] Sword Trace
  (`KismetSystemLibrary.K2_ClearAndInvalidateTimerHandle` (`self.Sword_Trace_Loop`)))

(event `Sphere Trace`
  (bind _returnvalue (`SceneComponent.K2_GetComponentLocation` (`self.Sphere Trace posi`)))
  ;[1 0.3372 0.3372] Sphere Trace: stab&kick
  (bind (_outhit _returnvalue_2) (`KismetSystemLibrary.SphereTraceSingle` :`Start` _returnvalue :`End` _returnvalue :`Radius` 25.0 :`TraceChannel` "TraceTypeQuery1" :`DrawDebugType` "ForDuration"))
  (if _returnvalue_2
    (bind (_bblockinghit _binitialoverlap _time _distance _location _impactpoint _normal _impactnormal _physmat _hitactor) (`GameplayStatics.BreakHitResult` _outhit))
    (`GameplayStatics.ApplyDamage` _hitactor 10.0)
    (`GameplayStatics.PlayWorldCameraShake` "/Game/Base_data/BP_CameraShake_受击.BP_CameraShake_受击_C" _location 0.0 2000.0)
    (`self.Play Sword hit sound`)
    (`GameplayStatics.SpawnEmitterAtLocation` "/Game/Effect_Particle/Particles/Blood/P_Blood_Splat_Cone.P_Blood_Splat_Cone" _location (`KismetMathLibrary.MakeRotFromXY` _normal _normal) (0.4 0.4 0.4) true "AutoRelease")))

(event `Play Sword hit sound`
  ;[1 1 1] Play Sword Hit Sound
  (`GameplayStatics.PlaySoundAtLocation` "/Game/Audio/剑击中音效/MS_Sword_hit.MS_Sword_hit" (`self.K2_GetActorLocation` (`self.GetOwner`)) (struct) 1.0 1.0 0.0 "/Game/Audio/SA_Character.SA_Character" null null null))

(event `Investigation Icon`
  (bind _investigate_widget (`self.investigate_Widget`))
  (`/Engine/EditorBlueprintResources/StandardMacros.FlipFlop`
    (:`A`
      (`SceneComponent.SetVisibility` _investigate_widget true false))
    (:`B`
      (`SceneComponent.SetVisibility` _investigate_widget false false))))

(fn `Attack`
  (returns (AnimationTime :type "Float (double-precision)"))
  (`self.SwordAttackFromBT_AI`)
  (return 0.4))

(fn `Stealth Back Assasin`
  (returns (`Ref Location` :type "Vector Structure") (`Assasin Rotation` :type "Rotator Structure"))
  (`self.PlayAnimMontage` "/Game/Characters/RPG_Characters/Animation/Assasination/Paired_Knife_Stealth_KidneyAndNeck_Vic1_Montage.Paired_Knife_Stealth_KidneyAndNeck_Vic1_Montage")
  (`self.Regdoll`)
  (`SceneComponent.SetVisibility` (`self.Assasinate Widget`) false false)
  (`SceneComponent.SetVisibility` (`self.Health Bar Widget`) false false)
  (return (`SceneComponent.K2_GetComponentLocation` (`self.Assasin Ref`)) (`self.K2_GetActorRotation`)))

(fn `UserConstructionScript`)