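; AI controller that starts the BT_AI behavior tree and turns sight and hearing perception into blackboard data.
; Successful sight sets Target Actor; lost sight or any non-sight stimulus clears it.
; When the controller is a BP_AI_Controller_Boss, these changes also activate or deactivate the boss.
; Hearing writes the stimulus location to Investigation Loc and calls InvestigationIcon on the controlled BP_AI pawn.
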(event `self.ReceiveBeginPlay`
  (`self.RunBehaviorTree` "/Game/AI/BT_AI.BT_AI"))

(event `self.AIPerception.OnTargetPerceptionUpdated`
  (params (Actor :type "Actor Object Reference") (Stimulus :type "AIStimulus Structure"))
  ;[1 1 1] 查看&追逐function
  (`self.SightDetect` Actor Stimulus)
  (`self.HearingDetect` Actor Stimulus))

(fn `HearingDetect`
  (params (Actor :type "Actor Object Reference") (Stimulus :type "AIStimulus Structure"))
  (bind _returnvalue (`AIPerceptionSystem.GetSenseClassForStimulus` Stimulus))
  (if (== _returnvalue "/Script/AIModule.AISense_Hearing")
    (`BlackboardComponent.SetValueAsVector` (`AIBlueprintHelperLibrary.GetBlackboard` null) "Investigation Loc" (`.StimulusLocation` (break `AIStimulus` Stimulus)))
    (bind _asbp_ai (cast `/Game/AI/BP_AI` (`self.K2_GetPawn`)))
    (`/Game/AI/BP_AI.Investigation Icon` _asbp_ai)))

(fn `SightDetect`
  (params (actor :type "Actor Object Reference") (stimulus :type "AIStimulus Structure"))
  (bind _returnvalue (`AIPerceptionSystem.GetSenseClassForStimulus` stimulus))
  (if (== _returnvalue "/Script/AIModule.AISense_Sight")
    (if (`.bSuccessfullySensed` (break `AIStimulus` stimulus))
      (`BlackboardComponent.SetValueAsObject` (`AIBlueprintHelperLibrary.GetBlackboard` null) "Target Actor" actor)
      (bind _asbp_ai_controller_boss (cast `/Game/AI/Boss/BP_AI_Controller_Boss` self))
      (`/Game/AI/Boss/BP_AI_Controller_Boss.Activate_Boss` _asbp_ai_controller_boss)
      (else
        (`BlackboardComponent.SetValueAsObject` (`AIBlueprintHelperLibrary.GetBlackboard` null) "Target Actor" null :!label _label)
        (bind _asbp_ai_controller_boss_2 (cast `/Game/AI/Boss/BP_AI_Controller_Boss` self))
        (`/Game/AI/Boss/BP_AI_Controller_Boss.Deactivate_Boss` _asbp_ai_controller_boss_2)))
    (else
      (goto _label))))

(fn `UserConstructionScript`)